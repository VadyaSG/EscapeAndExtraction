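; Main game mode that drives enemy spawning with rising difficulty and tracks the score.
; BeginPlay caches spawn delay and difficulty settings from getter functions.
; ActivateAllSpawners starts every BP_EnemySpawner and a looping timer that shortens the shared delay by a step without passing the minimum, then pushes it to all spawners.
; AddScore increments the score and updates the score widget.
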(event `ActivateAllSpawners`
  (bind _outactors (`GameplayStatics.GetAllActorsOfClass` "/Game/Main/Enemy/Blueprint/BP_EnemySpawner.BP_EnemySpawner_C"))
  (for _array_element _outactors
    (`/Game/Main/Enemy/Blueprint/BP_EnemySpawner.StartSpawn` _array_element (`self.CurrentSpawnDelay`)))
  (`KismetSystemLibrary.K2_SetTimerDelegate` (delegate `GlobalDifficultyTick`) (`self.DifficultUpdateIn`) true))

(event `self.ReceiveBeginPlay`
  (set `self.CurrentSpawnDelay` (`GameSettings.get_spawn_delay`))
  (set `self.DifficultyStep` (`GameSettings.get_dificulty_step`))
  (set `self.MinSpawnDelay` (`GameSettings.get_min_spawn_delay`))
  (set `self.DifficultUpdateIn` (`GameSettings.get_update_difficulty_time`)))

(event `GlobalDifficultyTick`
  (if (>= (- (`self.CurrentSpawnDelay`) (`self.DifficultyStep`)) (`self.MinSpawnDelay`))
    (bind _output_get (set `self.CurrentSpawnDelay` (- (`self.CurrentSpawnDelay`) (`self.DifficultyStep`))))
    (bind _outactors (`GameplayStatics.GetAllActorsOfClass` "/Game/Main/Enemy/Blueprint/BP_EnemySpawner.BP_EnemySpawner_C"))
    (for _array_element _outactors
      (`/Game/Main/Enemy/Blueprint/BP_EnemySpawner.UpdateSpawnSpeed` _array_element _output_get))))

(event `AddScore`
  (bind _result (`/Engine/EditorBlueprintResources/StandardMacros.IncrementInt` (`self.Score`))
    (:`  `
      (bind _output_get (set `self.Score` _result))
      (`/Game/Main/WidgetAndHud/PlayerInterface/WB_Score.UpdateScoreUI` (`self.WB_ScoreRef`) _output_get))))

(fn `UserConstructionScript`)