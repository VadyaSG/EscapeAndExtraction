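; BP_ActivateKeyCard is a spinning key card pickup that activates its TargetDoor's console when CH_Player overlaps it, then destroys itself.
; On BeginPlay and on a looping TTL timer, it relocates to a random SpawnPoints actor.
; A box overlap check recursively rerolls points occupied by key cards.
; The final move picks randomly again, so its destination can differ from the checked point.
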(event `self.ReceiveTick`
  (params (DeltaSeconds :type "Float (single-precision)"))
  (bind (_rotation_roll _rotation_pitch _rotation_yaw) (`KismetMathLibrary.BreakRotator` (`self.Rotation`)))
  (`SceneComponent.K2_AddWorldRotation` (`self.DefaultSceneRoot`) (`KismetMathLibrary.MakeRotator` 0.0 0.0 (* DeltaSeconds _rotation_yaw)) false false))

(event `self.Box.OnComponentBeginOverlap`
  (params (OverlappedComponent :type "PrimitiveComponent Object Reference") (OtherActor :type "Actor Object Reference") (OtherComp :type "PrimitiveComponent Object Reference") (OtherBodyIndex :type Integer) (bFromSweep :type Boolean) (SweepResult :type "HitResult Structure (by ref)"))
  (bind _asch_player (cast `/Game/Main/Player/Blueprints/CH_Player` OtherActor))
  (if (== _asch_player OtherActor)
    (`/Game/Main/Activate/BP_OpenedDoor.ActivateDoorConsol` (`self.TargetDoor`))
    (`self.K2_DestroyActor`)))

(event `self.ReceiveBeginPlay`
  (`self.SwitchPosInWorld`)
  (`KismetSystemLibrary.K2_SetTimerDelegate` (delegate `SwitchPosInWorld`) (`GameSettings.get_key_kard_ttl`) true))

(event `SwitchPosInWorld`
  (bind _spawnpoints (`self.SpawnPoints`))
  (bind _returnvalue (`self.K2_GetActorLocation` (`|GetArrayItem` _spawnpoints (`KismetMathLibrary.RandomIntegerInRange` 0 (`KismetArrayLibrary.Array_LastIndex` _spawnpoints)))))
  (if (> (`KismetArrayLibrary.Array_Length` _spawnpoints) 0)
    (bind _output_get (set `self.spawnPointLocation` _returnvalue))
    (bind (_outactors _returnvalue_2) (`KismetSystemLibrary.BoxOverlapActors` _output_get (57.0 57.0 57.0) (`|MakeArray` "ObjectTypeQuery2" :!type "EObjectTypeQuery Enum") "BP_ActivateKeyCard_C"))
    (if _returnvalue_2
      (`self.SwitchPosInWorld`)
      (else
        (`self.K2_SetActorLocation` _returnvalue)))))

(fn `UserConstructionScript`)