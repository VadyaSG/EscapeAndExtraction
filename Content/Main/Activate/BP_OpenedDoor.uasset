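; Door Blueprint that stays locked until a required number of consoles have been activated.
; Each ActivateDoorConsol call increments the activated count and pushes the saved quest text with current/max progress to the main HUD widget through BP_MainHud.
; Once the count reaches ConsolesToOpen it clears Locked, a check that only runs if the HUD cast succeeds.
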(event `ActivateDoorConsol`
  (bind _result (`/Engine/EditorBlueprintResources/StandardMacros.IncrementInt` (`self.activatedConsoles`))
    (:`  `
      (bind _asbp_main_hud (cast `/Game/Main/WidgetAndHud/MainHud/BP_MainHud` (`PlayerController.GetHUD` (`GameplayStatics.GetPlayerController` 0))))
      (message `/Game/Main/QuestTrigger/BPI_QuestInterface.UpdateQuest` (`/Game/Main/WidgetAndHud/MainHud/BP_MainHud.MainWidgetRef` _asbp_main_hud) (`|FormatText` "{MyText} {Current} /{Max}" (`self.SavedQuestText`) (`self.activatedConsoles`) (`self.ConsolesToOpen`)))
      (if (>= _result (`self.ConsolesToOpen`))
        (set `self.Locked` false)))))

(fn `UserConstructionScript`)