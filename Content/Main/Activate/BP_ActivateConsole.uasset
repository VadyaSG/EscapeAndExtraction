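; Interactable console that activates its linked TargetDoor once when the player presses Interact nearby.
; Overlapping the Box with CH_Player shows InteractionText and enables this actor's input for PlayerControllerMain.
; Leaving hides the text and calls DisableInput on the controller rather than on the console.
; Interacting sets IsActive to block repeats, swaps a mesh display material and calls ActivateDoorConsol on the door.
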(event `EnhancedInput|/Game/Main/Player/Input/AI_Interact`
  (params (ActionValue :type Boolean) (ElapsedSeconds :type "Float (double-precision)") (TriggeredSeconds :type "Float (double-precision)") (InputAction :type "InputAction Object Reference" :default "/Game/Main/Player/Input/AI_Interact.AI_Interact"))
  (:`Started`
    (if (not (`self.isActive`))
      (set `self.isActive` true)
      (`PrimitiveComponent.SetMaterial` (`self.StaticMesh`) 1 "/Game/SciFiWorld/Materials/MI_LabDisplay01B.MI_LabDisplay01B")
      (`PrimitiveComponent.SetMaterial` (`self.StaticMesh`) 1 "/Game/SciFiWorld/Materials/MI_LabDisplay01B.MI_LabDisplay01B")
      (`/Game/Main/Activate/BP_OpenedDoor.ActivateDoorConsol` (`self.TargetDoor`)))))

(event `self.Box.OnComponentBeginOverlap`
  (params (OverlappedComponent :type "PrimitiveComponent Object Reference") (OtherActor :type "Actor Object Reference") (OtherComp :type "PrimitiveComponent Object Reference") (OtherBodyIndex :type Integer) (bFromSweep :type Boolean) (SweepResult :type "HitResult Structure (by ref)"))
  (bind _asch_player (cast `/Game/Main/Player/Blueprints/CH_Player` OtherActor))
  (bind _asplayer_controller_main (cast `PlayerControllerMain` (`Pawn.GetController` _asch_player)))
  (`self.EnableInput` _asplayer_controller_main)
  (`SceneComponent.SetVisibility` (`self.InteractionText`) true false))

(event `self.Box.OnComponentEndOverlap`
  (params (OverlappedComponent :type "PrimitiveComponent Object Reference") (OtherActor :type "Actor Object Reference") (OtherComp :type "PrimitiveComponent Object Reference") (OtherBodyIndex :type Integer))
  (bind _asch_player (cast `/Game/Main/Player/Blueprints/CH_Player` OtherActor))
  (bind _asplayer_controller_main (cast `PlayerControllerMain` (`Pawn.GetController` _asch_player)))
  (`self.DisableInput` _asplayer_controller_main null)
  (`SceneComponent.SetVisibility` (`self.InteractionText`) false false))

(fn `UserConstructionScript`)