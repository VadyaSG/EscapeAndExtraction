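; BP_Enemy is an enemy with health, a world widget health bar and a pistol.
; On BeginPlay it caches the game mode, health bar widget and anim instance, then binds to its HealthComponent.
; Health changes update the bar's fill, turning it yellow then red as health drops, and death adds score through GM_MainGameMode.
; Tick syncs pistol visibility to the anim instance's has-weapon flag.
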(event `self.ReceiveTick`
  (params (DeltaSeconds :type "Float (single-precision)"))
  (bind _animref (`self.AnimRef`))
  (`/Engine/EditorBlueprintResources/StandardMacros.IsValid` _animref
    (:`Is Valid`
      (if (`/Game/Main/Enemy/Blueprint/ABP_Enemy.isHasWeapon` _animref)
        (bind _pistol (`self.Pistol`)
          (:`then`
            (`SceneComponent.SetVisibility` _pistol true false))
          (:`else`))
        (else
          (`SceneComponent.SetVisibility` (`self.Pistol`) false false))))))

(event `self.ReceiveBeginPlay`
  (bind _asgm_main_game_mode (cast `/Game/Main/GameMode/GM_MainGameMode` (`GameplayStatics.GetGameMode`)))
  (set `self.As GM Main Game Mode` _asgm_main_game_mode)
  (bind _aswb_enemy_health_bar (cast `/Game/Main/Enemy/Widget/WB_EnemyHealthBar` (`WidgetComponent.GetUserWidgetObject` (`self.hp_widget_comp`))))
  (set `self.As WB Enemy Health Bar` _aswb_enemy_health_bar)
  (add `HealthComponent.on_health_changed` (`self.health_component`) (delegate `HealthChanged`))
  (bind _asabp_enemy (cast `/Game/Main/Enemy/Blueprint/ABP_Enemy` (`SkeletalMeshComponent.GetAnimInstance` (`self.Mesh`))))
  (set `self.AnimRef` _asabp_enemy)
  (add `HealthComponent.on_death` (`self.health_component`) (delegate `addScore`)))

(event `HealthChanged`
  (params (current_hp :type "Float (single-precision)") (max_hp :type "Float (single-precision)"))
  (`self.ChangeHpBar` current_hp max_hp))

(event `addScore`
  (`/Game/Main/GameMode/GM_MainGameMode.AddScore` (`self.As GM Main Game Mode`)))

(fn `ChangeHpBar`
  (params (currentHp :type "Float (double-precision)") (MaxHp :type "Float (double-precision)"))
  (locals (percent :type "Float (double-precision)"))
  (bind _healthbar (`/Game/Main/Enemy/Widget/WB_EnemyHealthBar.HealthBar` (`self.As WB Enemy Health Bar`)))
  (bind _output_get (set `local.percent` (/ currentHp MaxHp)))
  (`ProgressBar.SetPercent` _healthbar _output_get)
  (if (<= (`local.percent`) 0.5)
    (`ProgressBar.SetFillColorAndOpacity` _healthbar (struct :`R` 1.0 :`G` 0.982393 :`B` 0.000761 :`A` 1.0))
    (if (<= (`local.percent`) 0.2)
      (`ProgressBar.SetFillColorAndOpacity` _healthbar (struct :`R` 0.598958 :`G` 0.013139 :`A` 1.0)))))

(fn `UserConstructionScript`)