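; BP_MillieEnemy is an enemy Blueprint that deals contact damage through its hands.
; On BeginPlay it scales Damage by an enemy modification factor and sets the HealthComponent's max HP to current HP times that factor.
; Overlaps on LeftHand1 and RightHand apply that damage to the other actor, skipping other BP_MillieEnemy instances.
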(event `self.ReceiveBeginPlay`
  (bind _health_component (`self.health_component`))
  (`parent.ReceiveBeginPlay`)
  (set `self.Damage` (* (`self.Damage`) (`GameSettings.GetEnemyModificationFactor`)))
  (set `HealthComponent.max_hp` (* (`HealthComponent.get_curren_hp` _health_component) (`GameSettings.GetEnemyModificationFactor`)) _health_component))

(event `self.LeftHand1.OnComponentBeginOverlap`
  (params (OverlappedComponent :type "PrimitiveComponent Object Reference") (OtherActor :type "Actor Object Reference") (OtherComp :type "PrimitiveComponent Object Reference") (OtherBodyIndex :type Integer) (bFromSweep :type Boolean) (SweepResult :type "HitResult Structure (by ref)"))
  (cast `/Game/Main/Enemy/Blueprint/BP_MillieEnemy` OtherActor
    (:`CastFailed`
      (`GameplayStatics.ApplyDamage` OtherActor (`self.Damage`)))))

(event `self.RightHand.OnComponentBeginOverlap`
  (params (OverlappedComponent :type "PrimitiveComponent Object Reference") (OtherActor :type "Actor Object Reference") (OtherComp :type "PrimitiveComponent Object Reference") (OtherBodyIndex :type Integer) (bFromSweep :type Boolean) (SweepResult :type "HitResult Structure (by ref)"))
  (cast `/Game/Main/Enemy/Blueprint/BP_MillieEnemy` OtherActor
    (:`CastFailed`
      (`GameplayStatics.ApplyDamage` OtherActor (`self.Damage`)))))

(fn `UserConstructionScript`
  (`parent.UserConstructionScript`))