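; Main player controller that autosaves the game on a looping timer and restores a saved game at startup.
; When the game instance flags a load, BeginPlay replaces all enemies with BP_Enemy spawns at saved transforms, restores player transform, health and score, then possesses the player.
; Autosave writes that state to one fixed slot and briefly shows a save widget.
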(event `self.ReceiveBeginPlay`
  (bind _as_ch_player (`self.As CH Player`))
  (`KismetSystemLibrary.K2_SetTimerDelegate` (delegate `Autosave`) 20.0 true)
  (bind _asch_player (cast `/Game/Main/Player/Blueprints/CH_Player` (`GameplayStatics.GetPlayerCharacter` 0)))
  (set `self.As CH Player` _asch_player)
  (bind _asgm_main_game_mode (cast `/Game/Main/GameMode/GM_MainGameMode` (`GameplayStatics.GetGameMode`)))
  (set `self.As GM Main Game Mode` _asgm_main_game_mode)
  (bind _asgi_main_game_instance (cast `/Game/Main/GameMode/GI_MainGameInstance` (`GameplayStatics.GetGameInstance`)))
  (if (`/Game/Main/GameMode/GI_MainGameInstance.IsGameLoad` _asgi_main_game_instance)
    (bind _returnvalue (`GameplayStatics.LoadGameFromSlot` (`/Game/Main/GameMode/GI_MainGameInstance.SlotToLoad ` _asgi_main_game_instance)))
    (bind _asbp_save_game (cast `/Game/Main/Saves/BP_SaveGame` _returnvalue))
    (bind _outactors (`GameplayStatics.GetAllActorsOfClass` "/Script/EscapeAndExtraction.BaseEnemy"))
    (for _array_element _outactors
      (`self.K2_DestroyActor` _array_element))
    (bind (_saveddata_playertransform _saveddata_currenthp _saveddata_score _saveddata_mobscount _saveddata_mobstransform) (break `/Game/Main/Saves/S_SavedData` (`/Game/Main/Saves/BP_SaveGame.SavedData` _asbp_save_game)))
    (for _array_element_2 _saveddata_mobstransform
      (`|SpawnActorFromClass` "/Game/Main/Enemy/Blueprint/BP_Enemy.BP_Enemy_C" _array_element_2 "Undefined" "MultiplyWithRoot" null false null))
    (`self.K2_SetActorTransform` _as_ch_player _saveddata_playertransform false false)
    (set `/Game/Main/GameMode/GM_MainGameMode.Score` _saveddata_score (`self.As GM Main Game Mode`))
    (`HealthComponent.set_curren_hp` (`MainCharacter.health_component` _as_ch_player) _saveddata_currenthp)
    (`self.Possess` (`GameplayStatics.GetPlayerCharacter` 0))
    (set `/Game/Main/GameMode/GI_MainGameInstance.IsGameLoad` false _asgi_main_game_instance)))

(event `Autosave`
  (bind _returnvalue (`GameplayStatics.CreateSaveGameObject` "/Game/Main/Saves/BP_SaveGame.BP_SaveGame_C"))
  (bind _outactors (`GameplayStatics.GetAllActorsOfClass` "/Script/EscapeAndExtraction.BaseEnemy"))
  (`KismetArrayLibrary.Array_Clear` (`self.mobpos`))
  (for _array_element _outactors
    (`KismetArrayLibrary.Array_Add` (`self.mobpos`) (`self.GetTransform` _array_element)))
  (set `/Game/Main/Saves/BP_SaveGame.SavedData` (make `/Game/Main/Saves/S_SavedData` (`self.GetTransform` (`GameplayStatics.GetPlayerCharacter` 0)) (`HealthComponent.get_curren_hp` (`MainCharacter.health_component` (`self.As CH Player`))) (`/Game/Main/GameMode/GM_MainGameMode.Score` (`self.As GM Main Game Mode`)) (`KismetArrayLibrary.Array_Length` _outactors) (`self.mobpos`)) _returnvalue)
  (`GameplayStatics.SaveGameToSlot` _returnvalue "slot")
  (bind _returnvalue_2 (`|CreateWidget` "/Game/Main/Saves/Widget/WB_SaveGame.WB_SaveGame_C"))
  (`UserWidget.AddToViewport` _returnvalue_2 0)
  (`KismetSystemLibrary.Delay` 2.0)
  (`Widget.RemoveFromParent` _returnvalue_2))

(fn `UserConstructionScript`)