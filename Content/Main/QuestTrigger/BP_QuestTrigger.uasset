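; Quest trigger volume that updates the HUD quest message when the player enters its box, adding console progress if a Door is linked.
; Overlap also stores the text on that Door and the first BP_OpenedDoor found.
; The player's first exit plays a quest sound through GM_MainGameMode.
; It also listens to game mode time updates, switching the message to "Jump on teleport" at one second or less.
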(event `self.ReceiveBeginPlay`
  (bind _asgm_main_game_mode (cast `/Game/Main/GameMode/GM_MainGameMode` (`GameplayStatics.GetGameMode`)))
  (set `self.As GM Main Game Mode` _asgm_main_game_mode)
  (bind _asch_player (cast `/Game/Main/Player/Blueprints/CH_Player` (`GameplayStatics.GetPlayerCharacter` 0)))
  (bind _asbp_main_hud (cast `/Game/Main/WidgetAndHud/MainHud/BP_MainHud` (`PlayerController.GetHUD` (`PlayerState.GetPlayerController` (`Pawn.PlayerState` _asch_player)))))
  (add `/Game/Main/GameMode/GM_MainGameMode.OnTimeUpdated` (`self.As GM Main Game Mode`) (delegate `UpdateQuestFromTime`)))

(event `UpdateQuestFromTime`
  (params (CurrentSeconds :type "Float (double-precision)"))
  (if (<= CurrentSeconds 1.0)
    (bind _mainwidgetref (`/Game/Main/WidgetAndHud/MainHud/BP_MainHud.MainWidgetRef` (stale `self.ReceiveBeginPlay` _asbp_main_hud))
      (:`then`
        (message `/Game/Main/QuestTrigger/BPI_QuestInterface.UpdateQuest` _mainwidgetref "Jump on teleport"))
      (:`else`))))

(event `self.Box.OnComponentBeginOverlap`
  (params (OverlappedComponent :type "PrimitiveComponent Object Reference") (OtherActor :type "Actor Object Reference") (OtherComp :type "PrimitiveComponent Object Reference") (OtherBodyIndex :type Integer) (bFromSweep :type Boolean) (SweepResult :type "HitResult Structure (by ref)"))
  (bind _door (`self.Door`))
  (bind _door_2 (`self.Door`))
  (`/Engine/EditorBlueprintResources/StandardMacros.IsValid` _door_2
    (:`Is Valid`
      (set `/Game/Main/Activate/BP_OpenedDoor.SavedQuestText` (`self.TextToShow`) _door_2))
    (:`Is Not Valid`
      _))
  (bind _asch_player (cast `/Game/Main/Player/Blueprints/CH_Player` OtherActor))
  (set `self.As CH Player` _asch_player)
  (bind _returnvalue (`GameplayStatics.GetActorOfClass` "/Game/Main/Activate/BP_OpenedDoor.BP_OpenedDoor_C"))
  (set `/Game/Main/Activate/BP_OpenedDoor.SavedQuestText` (`self.TextToShow`) _returnvalue)
  (bind _asbp_main_hud (cast `/Game/Main/WidgetAndHud/MainHud/BP_MainHud` (`PlayerController.GetHUD` (`PlayerState.GetPlayerController` (`Pawn.PlayerState` _asch_player)))))
  (`/Engine/EditorBlueprintResources/StandardMacros.IsValid` (`self.Door`)
    (:`Is Valid`
      (bind _mainwidgetref (`/Game/Main/WidgetAndHud/MainHud/BP_MainHud.MainWidgetRef` _asbp_main_hud))
      (message `/Game/Main/QuestTrigger/BPI_QuestInterface.UpdateQuest` _mainwidgetref (`|FormatText` "{Text} {min}/{max}" (`self.TextToShow`) (`/Game/Main/Activate/BP_OpenedDoor.activatedConsoles` _door) (`/Game/Main/Activate/BP_OpenedDoor.ConsolesToOpen` _door))))
    (:`Is Not Valid`
      (message `/Game/Main/QuestTrigger/BPI_QuestInterface.UpdateQuest` _mainwidgetref (`self.TextToShow`)))))

(event `self.Box.OnComponentEndOverlap`
  (params (OverlappedComponent :type "PrimitiveComponent Object Reference") (OtherActor :type "Actor Object Reference") (OtherComp :type "PrimitiveComponent Object Reference") (OtherBodyIndex :type Integer))
  (if (== OtherActor (`self.As CH Player`))
    (if (not (`self.is triggered`))
      (`/Game/Main/GameMode/GM_MainGameMode.playQuestSound` (`self.As GM Main Game Mode`) (`self.sound`))
      (set `self.is triggered` true))))

(fn `UpdateQuest`
  (params (TextQuest :type Text))
  (return))

(fn `UserConstructionScript`)