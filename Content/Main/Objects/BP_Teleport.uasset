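; BP_Teleport is a level exit actor that gates a win trigger behind a survival timer.
; When CH_Player enters TimerTrigger, it shows WB_Timer, binds to GM_MainGameMode's time updates, starts survival time and destroys the trigger.
; When the reported seconds reach zero, it destroys the Door, removes the timer widget and unbinds the update event.
; Any overlap with Box pauses the game and shows WB_WonMenu, with no player check.
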(event `self.ReceiveBeginPlay`
  (bind _asgm_main_game_mode (cast `/Game/Main/GameMode/GM_MainGameMode` (`GameplayStatics.GetGameMode`)))
  (set `self.As GM Main Game Mode` _asgm_main_game_mode))

(event `self.Box.OnComponentBeginOverlap`
  (params (OverlappedComponent :type "PrimitiveComponent Object Reference") (OtherActor :type "Actor Object Reference") (OtherComp :type "PrimitiveComponent Object Reference") (OtherBodyIndex :type Integer) (bFromSweep :type Boolean) (SweepResult :type "HitResult Structure (by ref)"))
  (`GameplayStatics.SetGamePaused` true)
  (bind _returnvalue (`|CreateWidget` "/Game/Main/WidgetAndHud/GameStateWidgets/WB_WonMenu.WB_WonMenu_C"))
  (`UserWidget.AddToViewport` _returnvalue 0))

(event `self.TimerTrigger.OnComponentBeginOverlap`
  (params (OverlappedComponent :type "PrimitiveComponent Object Reference") (OtherActor :type "Actor Object Reference") (OtherComp :type "PrimitiveComponent Object Reference") (OtherBodyIndex :type Integer) (bFromSweep :type Boolean) (SweepResult :type "HitResult Structure (by ref)"))
  (bind _as_gm_main_game_mode (`self.As GM Main Game Mode`))
  (cast `/Game/Main/Player/Blueprints/CH_Player` OtherActor)
  (bind _returnvalue (`|CreateWidget` "/Game/Main/WidgetAndHud/PlayerInterface/WB_Timer.WB_Timer_C"))
  (`UserWidget.AddToViewport` _returnvalue 0)
  (add `/Game/Main/GameMode/GM_MainGameMode.OnTimeUpdated` _as_gm_main_game_mode (delegate `TimeOut`))
  (`/Game/Main/GameMode/GM_MainGameMode.StartSurvivalTime` _as_gm_main_game_mode)
  (`ActorComponent.K2_DestroyComponent` (`self.TimerTrigger`)))

(event `TimeOut`
  (params (CurrentSeconds :type "Float (double-precision)"))
  (if (<= CurrentSeconds 0.0)
    (`ActorComponent.K2_DestroyComponent` (`self.door`))
    (`Widget.RemoveFromParent` (stale `self.TimerTrigger.OnComponentBeginOverlap` _returnvalue))
    (clear `/Game/Main/GameMode/GM_MainGameMode.OnTimeUpdated` (`self.As GM Main Game Mode`))))

(fn `UserConstructionScript`)