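; BP_MainHud is the main HUD Blueprint that creates the in-game, pause and game-over UI.
; On BeginPlay it adds WBP_MainWidget to the viewport, hands its score widget to GM_MainGameMode, and pre-creates a hidden pause widget.
; It binds to the MainCharacter HealthComponent's OnDeath, which shows the game-over widget after a configurable delay.
; The pause widget is only created after the game mode and character casts succeed.
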(event `self.ReceiveBeginPlay`
  (bind _returnvalue (`|CreateWidget` "/Game/Main/WidgetAndHud/PlayerInterface/WBP_MainWidget.WBP_MainWidget_C"))
  (bind _output_get (set `self.MainWidgetRef` _returnvalue))
  (`UserWidget.AddToViewport` _output_get 0)
  (bind _asgm_main_game_mode (cast `/Game/Main/GameMode/GM_MainGameMode` (`GameplayStatics.GetGameMode`)))
  (set `/Game/Main/GameMode/GM_MainGameMode.WB_ScoreRef` (`/Game/Main/WidgetAndHud/PlayerInterface/WBP_MainWidget.WB_Score` (`self.MainWidgetRef`)) _asgm_main_game_mode)
  (bind _asmain_character (cast `MainCharacter` (`UserWidget.GetOwningPlayerPawn` (`self.MainWidgetRef`))))
  (bind _output_get_2 (set `self.As Main Character` _asmain_character))
  (add `HealthComponent.on_death` (`MainCharacter.health_component` _output_get_2) (delegate `OpenGameOverMenu`))
  (bind _returnvalue_2 (`|CreateWidget` "/Game/Main/WidgetAndHud/GameStateWidgets/WB_Pause.WB_Pause_C"))
  (bind _output_get_3 (set `self.PauseWbRef` _returnvalue_2))
  (`Widget.SetVisibility` _output_get_3 "Hidden")
  (`UserWidget.AddToViewport` _returnvalue_2 0))

(event `OpenGameOverMenu`
  (`KismetSystemLibrary.Delay` (`self.DelayBeforeSpawnGMWidget`))
  (bind _returnvalue (`|CreateWidget` "/Game/Main/WidgetAndHud/GameStateWidgets/WB_GameOver.WB_GameOver_C"))
  (`UserWidget.AddToViewport` _returnvalue 0))

(fn `UserConstructionScript`)